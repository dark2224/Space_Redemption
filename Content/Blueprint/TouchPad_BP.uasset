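; Touchpad interactable that the pilot pawn's right hand grabs and slides across to drive a 2D mapping coordinate.
; Tick runs an Idle/Approaching/Interacting state machine, entered when the hand overlaps ApproachDetector.
; The desired hand pose follows the hand projected onto the pad's plane, and grabbing within the activation radius starts interaction.
; While held, real-hand movement along the actor's forward and right axes accumulates, scaled and clamped, into that coordinate.
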(event OnComponentBeginOverlap(ApproachDetector)
  (params (OverlappedComponent :type Primitive%20Component%20Object%20Reference) (OtherActor :type Actor%20Object%20Reference) (OtherComp :type Primitive%20Component%20Object%20Reference) (OtherBodyIndex :type Integer) (bFromSweep :type Boolean) (SweepResult :type Hit%20Result%20Structure%20%28by%20ref%29))
  (|Approach상태초기화 OtherComp OtherComp OtherComp))

(event EventBeginPlay
  (Class|TangibleActor|SetDesiredHandTransform (Variables|Default|GetDesiredHandScene))
  (Variables|Default|SetInteractingAnimation "/Game/Model/Player/RightAnim/anim_touchpad_idle.anim_touchpad_idle"))

(event EventTick
  (params (DeltaSeconds :type Float%20%28single-precision%29))
  (bind _returnvalue (Class|TangibleActor|GetStaus))
  (switch Utilities|FlowControl|Switch|SwitchonInteractionStatus _returnvalue
    (:Idle
      (|Idle))
    (:Approaching
      (|접근중조건확인))
    (:Interacting
      (|상호작용중))))

(fn ConstructionScript
  (Class|TouchPad|SetSound (Variables|Default|Getgunsound) (Variables|Default|Getgunsoud%28End%29)))

(fn RelocateDesiredHandScene(Scene)
  (params (손 :type Scene%20Component%20Object%20Reference))
  (bind _newlocation (CallFunction|RelocateDesiredHandScene(WithVector) (Transformation|GetWorldLocation 손)))
  (return _newlocation))

(fn DistanceBetweenHand&DesiredHand
  (bind _returnvalue (Class|TangibleActor|GetTargetHand))
  (return (Math|Vector|VectorLength (- (Transformation|GetWorldLocation _returnvalue) (Transformation|GetWorldLocation (Variables|Default|GetDesiredHandScene))))))

(fn RelocateDesiredHandScene(WithVector)
  (params (TargetLocation :type Vector))
  (bind _origin (Variables|컴포넌트|GetOrigin))
  (bind _desiredhandscene (Variables|Default|GetDesiredHandScene))
  (bind _returnvalue (Transformation|GetWorldRotation _origin))
  (bind _returnvalue_2 (Transformation|GetWorldLocation _origin))
  (bind _relativelocation (Variables|/Script/Engine.SceneComponent|GetRelativeLocation _desiredhandscene))
  (bind _z (Math|Vector|BreakVector _relativelocation))
  (bind _returnvalue_3 (Math|Vector|GetUpVector _returnvalue))
  (bind _returnvalue_4 (Class|KismetMathLibrary|ProjectPointontoPlane TargetLocation _returnvalue_2 _returnvalue_3))
  (bind _returnvalue_5 (* _returnvalue_3 _z))
  (bind _returnvalue_6 (+ _returnvalue_5 _returnvalue_4))
  (Transformation|SetWorldLocation (Variables|Default|GetDesiredHandScene) _returnvalue_6 false false)
  (return _returnvalue_6))