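; BP_UFO is an enemy UFO that shows booster exhaust and disappears on death.
; Each Tick, when BoosterDelay returns true, it spawns P_Boost emitters at left and right StaticMesh booster sockets while HP is above zero.
; Actor overlap calls SetDamage with zero, then Damage, which sets the DEATH type, hides the actor and disables Box collision if HP is below zero.
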(event EventBeginPlay)

(event Collision|EventActorBeginOverlap
  (params (OtherActor :type Actor%20Object%20Reference))
  (Utilities|Set|Damage)
  (CallFunction|Damage))

(event EventTick
  (params (DeltaSeconds :type Float%20%28single-precision%29))
  (bind _returnvalue (Class|Enemy|BoosterDelay))
  (if _returnvalue
    (CallFunction|RightBooster)
    (CallFunction|LeftBooster)))

(fn ConstructionScript)

(fn RightBooster
  (bind _returnvalue (Class|Enemy|GetHp))
  (if (> _returnvalue 0)
    (Effects|SpawnEmitteratLocation "/Game/Particles/Bosster/P_Boost.P_Boost" (Transformation|GetSocketLocation (Variables|Default|GetStaticMesh) "RightUPBooster") "-90.000000, 0, 0")
    (Effects|SpawnEmitteratLocation "/Game/Particles/Bosster/P_Boost.P_Boost" (Transformation|GetSocketLocation (Variables|Default|GetStaticMesh) "RightDownBooster") "-90.000000, 0, 0")))

(fn Damage
  (bind _returnvalue (Class|Enemy|GetHp))
  (if (< _returnvalue 0)
    (Utilities|Set|EnemyType "ENEMY_DEATH")
    (Rendering|SetActorHiddenInGame true)
    (Collision|SetCollisionEnabled (Variables|Default|GetBox) "NoCollision")))

(fn LeftBooster
  (bind _returnvalue (Class|Enemy|GetHp))
  (if (> _returnvalue 0)
    (Effects|SpawnEmitteratLocation "/Game/Particles/Bosster/P_Boost.P_Boost" (Transformation|GetSocketLocation (Variables|Default|GetStaticMesh) "LeftUPBooster") "90.000000, 0, 0")
    (Effects|SpawnEmitteratLocation "/Game/Particles/Bosster/P_Boost.P_Boost" (Transformation|GetSocketLocation (Variables|Default|GetStaticMesh) "LeftDownBooster") "90.000000, 0, 0")))