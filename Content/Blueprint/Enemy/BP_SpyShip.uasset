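; BP_SpyShip is an enemy spy ship that takes damage on contact and shows booster exhaust while alive.
; Each overlap applies 1 damage, then hides the ship and disables its Box collision once HP drops below zero, without destroying the actor.
; Tick spawns boost particles at the left and right booster sockets whenever HP is positive and BoosterDelay allows it.
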(event EventBeginPlay)

(event Collision|EventActorBeginOverlap
  (params (OtherActor :type Actor%20Object%20Reference))
  (Utilities|Set|Damage 1)
  (CallFunction|Damage))

(event EventTick
  (params (DeltaSeconds :type Float%20%28single-precision%29))
  (CallFunction|Booster))

(fn ConstructionScript)

(fn Booster
  (bind _returnvalue (Class|Enemy|GetHp))
  (if (> _returnvalue 0)
    (bind _returnvalue_2 (Class|Enemy|BoosterDelay))
    (if _returnvalue_2
      (Effects|SpawnEmitteratLocation "/Game/Particles/Booster/P_Boost.P_Boost" (Transformation|GetSocketLocation (Variables|Default|GetStaticMesh) "RightBooster") (Transformation|GetActorRotation))
      (Effects|SpawnEmitteratLocation "/Game/Particles/Booster/P_Boost.P_Boost" (Transformation|GetSocketLocation (Variables|Default|GetStaticMesh) "LeftBooster") (Transformation|GetActorRotation)))))

(fn Damage
  (bind _returnvalue (Class|Enemy|GetHp))
  (if (< _returnvalue 0)
    (Rendering|SetActorHiddenInGame true)
    (Collision|SetCollisionEnabled (Variables|Default|GetBox) "NoCollision")))