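; BP_Alliance is an allied unit actor that fires BP_Missile while it has health.
; Each tick with HP above zero, it unhides itself and, when the shoot flag and delay check pass, spawns a missile at the mesh's "Shoot" socket, passing Position and Angle.
; Overlaps call SetDamage with zero, then hide the actor and disable box collision if HP is negative.
; Booster only reads HP.
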(event EventBeginPlay)

(event Collision|EventActorBeginOverlap
  (params (OtherActor :type Actor%20Object%20Reference))
  (Utilities|Set|Damage)
  (CallFunction|Damage))

(event EventTick
  (params (DeltaSeconds :type Float%20%28single-precision%29))
  (CallFunction|Booster)
  (bind _returnvalue (Class|Alliance|GetHp))
  (if (> _returnvalue 0)
    (Rendering|SetActorHiddenInGame false)
    (CallFunction|Battle)))

(fn ConstructionScript)

(fn Booster
  (Class|Alliance|GetHp))

(fn Damage
  (bind _returnvalue (Class|Alliance|GetHp))
  (if (< _returnvalue 0)
    (Rendering|SetActorHiddenInGame true)
    (Collision|SetCollisionEnabled (Variables|Default|GetBox) "NoCollision")))

(fn Battle
  (bind _returnvalue (Class|Alliance|GetShoot))
  (if _returnvalue
    (bind _returnvalue_2 (Class|Alliance|ShootDelay))
    (if _returnvalue_2
      (bind _returnvalue_3 (Game|SpawnActorfromClass "/Game/Blueprint/Missile/BP_Missile.BP_Missile_C" (Math|Conversions|ToTransform(Vector) (Transformation|GetSocketLocation (Variables|Default|GetStaticMesh) "Shoot")) "Undefined" 0 0))
      (Utilities|Set|StartCheck _returnvalue_3 true)
      (Variables|/Game/Blueprint/Missile/BP_Missile.BP_Missile_C|SetPosition _returnvalue_3 (Variables|Calculation|GetPosition))
      (Variables|/Game/Blueprint/Missile/BP_Missile.BP_Missile_C|SetAngle _returnvalue_3 (Variables|Calculation|GetAngle)))))