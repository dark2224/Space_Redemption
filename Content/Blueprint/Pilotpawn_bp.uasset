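; Pilot pawn with left and right motion-tracked hands, apparently for VR.
; On BeginPlay it initializes each hand through DefaultSet, passing that hand's collision and a separate "real hand" collision.
; Unconnected nodes, which never run, would copy tracked controller positions to the real-hand scene components and print the left one.
; Tick, overlap and construction logic are empty.
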(event EventBeginPlay
  (Class|Hand|DefaultSet (Variables|Default|GetRightHand) (Variables|Default|GetRightHandCollision) (Variables|Default|GetRightRealHandcollision))
  (Class|Hand|DefaultSet (Variables|Default|GetLeftHand) (Variables|Default|GetLeftHandCollision) (Variables|Default|GetLeftRealHandCollision)))

(event Collision|EventActorBeginOverlap
  (params (OtherActor :type Actor%20Object%20Reference)))

(event EventTick
  (params (DeltaSeconds :type Float%20%28single-precision%29)))

(event Input|ActionEvents|InputActionMissile
  (params (Key :type Key%20Structure :default "AnyKey")))

(event Input|ActionEvents|InputActionGuidedMissile
  (params (Key :type Key%20Structure :default "AnyKey")))

(fn ConstructionScript)