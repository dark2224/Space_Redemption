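; BP_Missile is a missile actor that shows a booster trail and hides and resets itself on overlap.
; On BeginPlay it spawns a persistent fireball emitter, which Tick moves to the mesh's Booster socket and unhides whenever BoosterDelay returns true.
; On overlap it spawns a hit effect, hides actor and trail, disables box collision, calls ResetMissile and clears the start check, rather than destroying the actor.
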(event EventBeginPlay
  (CallFunction|Initialize))

(event Collision|EventActorBeginOverlap
  (params (OtherActor :type Actor%20Object%20Reference))
  (CallFunction|Collision))

(event EventTick
  (params (DeltaSeconds :type Float%20%28single-precision%29))
  (CallFunction|Booster))

(fn ConstructionScript)

(fn Booster
  (bind _particle (Variables|Default|GetParticle))
  (bind _returnvalue (Class|Missile|BoosterDelay))
  (if _returnvalue
    (Transformation|SetWorldLocation _particle (Transformation|GetSocketLocation (Variables|Default|GetStaticMesh) "Booster") false false)
    (Development|SetHiddeninGame _particle false false)))

(fn Initialize
  (bind _returnvalue (Effects|SpawnEmitteratLocation "/Game/Particles/RockBooster/P_Fireball_Projectile.P_Fireball_Projectile" "0, 0, 0" "0.000000,0.000000,0.000000" false))
  (Variables|Default|SetParticle _returnvalue))

(fn Collision
  (Effects|SpawnEmitteratLocation "/Game/Particles/Hit/P_HitParticle.P_HitParticle" (Transformation|GetActorLocation))
  (Rendering|SetActorHiddenInGame true)
  (Class|Missile|ResetMissile)
  (Development|SetHiddeninGame (Variables|Default|GetParticle) true false)
  (Collision|SetCollisionEnabled (Variables|Default|GetBox) "NoCollision")
  (Utilities|Set|StartCheck false))