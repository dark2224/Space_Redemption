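; Guided missile actor that shows a booster trail in flight and an explosion effect on overlap, then resets for reuse.
; BeginPlay hides the actor and pre-spawns a hidden fireball emitter, which Tick reveals and moves to the mesh's Booster socket once the start and delay checks pass.
; Overlap spawns a hit effect, hides missile and trail, calls ResetMissile and disables box collision.
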(event EventBeginPlay
  (CallFunction|Initialize))

(event Collision|EventActorBeginOverlap
  (params (OtherActor :type Actor%20Object%20Reference))
  (CallFunction|Collision))

(event EventTick
  (params (DeltaSeconds :type Float%20%28single-precision%29))
  (CallFunction|Booster))

(fn ConstructionScript)

(fn Booster
  (bind _particle (Variables|Particle|GetParticle))
  (bind _returnvalue (Class|Missile|GetStartCheck))
  (if _returnvalue
    (bind _returnvalue_2 (Class|Missile|BoosterDelay))
    (if _returnvalue_2
      (Transformation|SetWorldLocation _particle (Transformation|GetSocketLocation (Variables|Default|GetStaticMesh) "Booster") false false)
      (Development|SetHiddeninGame _particle false false))))

(fn Collision
  (Effects|SpawnEmitteratLocation "/Game/Particles/Hit/P_HitParticle.P_HitParticle" (Transformation|GetActorLocation))
  (Rendering|SetActorHiddenInGame true)
  (Class|Missile|ResetMissile)
  (Development|SetHiddeninGame (Variables|Particle|GetParticle) true false)
  (Collision|SetCollisionEnabled (Variables|Default|GetBox) "NoCollision"))

(fn Initialize
  (Rendering|SetActorHiddenInGame true)
  (bind _returnvalue (Effects|SpawnEmitteratLocation "/Game/Particles/RockBooster/P_Fireball_Projectile.P_Fireball_Projectile" "0.000000,0.000000,1000.000000" "0.000000,0.000000,0.000000" false))
  (bind _output_get (Variables|Particle|SetParticle _returnvalue))
  (Development|SetHiddeninGame _output_get true false))