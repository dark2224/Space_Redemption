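; Pushable button for the PilotPawn's virtual hand, built on inherited hand-interaction states; only the left hand engages it.
; An ApproachDetector overlap starts approaching, and Tick switches to interacting once the hand is close and wants to grab.
; The hand's distance from the actor's plane drives DesiredHandScene and button height, limiting button travel between push markers.
; While interacting, the real-world hand drives the press until leaving the detector; grab release is ignored.
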(event OnComponentBeginOverlap(ApproachDetector)
  (params (OverlappedComponent :type Primitive%20Component%20Object%20Reference) (OtherActor :type Actor%20Object%20Reference) (OtherComp :type Primitive%20Component%20Object%20Reference) (OtherBodyIndex :type Integer) (bFromSweep :type Boolean) (SweepResult :type Hit%20Result%20Structure%20%28by%20ref%29))
  (|Approach상태초기화 OtherComp OtherComp OtherComp))

(event EventBeginPlay
  (Class|TangibleActor|SetDesiredHandTransform (Variables|Default|GetDesiredHandScene))
  (Variables|Default|SetInteractingAnimation "/Game/Model/Player/LeftAnim/anim_button_idle.anim_button_idle"))

(event EventTick
  (params (DeltaSeconds :type Float%20%28single-precision%29))
  (bind _returnvalue (Class|TangibleActor|GetStaus))
  (switch Utilities|FlowControl|Switch|SwitchonInteractionStatus _returnvalue
    (:Idle
      (|Idle))
    (:Approaching
      (|접근중조건확인))
    (:Interacting
      (|상호작용중))))

(fn ConstructionScript
  (Variables|Default|SetMoveLength (Math|Vector|VectorLength (- (Variables|/Script/Engine.SceneComponent|GetRelativeLocation (Variables|Default|GetWherePushStarts)) (Variables|/Script/Engine.SceneComponent|GetRelativeLocation (Variables|Default|GetWherePushEnds)))))
  (Variables|Default|SetRelativeButtonZ (.Z (Math|Vector|BreakVector (Variables|/Script/Engine.SceneComponent|GetRelativeLocation (Variables|Default|GetButton))))))

(fn ReloacteDesiredHandScene
  (params (타겟 :type Hand%20Object%20Reference))
  (CallFunction|ReloacteDesiredHandScene2 (Transformation|GetWorldLocation 타겟)))

(fn ReloacteDesiredHandScene2
  (params (TargetPoint :type Vector))
  (bind _desiredhandscene (Variables|Default|GetDesiredHandScene))
  (bind _wherepushstarts (Variables|Default|GetWherePushStarts))
  (bind _button (Variables|Default|GetButton))
  (bind _desiredhandscene_2 (Variables|Default|GetDesiredHandScene))
  (bind _desiredhandscene_3 (Variables|Default|GetDesiredHandScene))
  (bind _relativelocation (Variables|/Script/Engine.SceneComponent|GetRelativeLocation _desiredhandscene))
  (bind _relativelocation_2 (Variables|/Script/Engine.SceneComponent|GetRelativeLocation _wherepushstarts))
  (bind _relativelocation_3 (Variables|/Script/Engine.SceneComponent|GetRelativeLocation _button))
  (bind _relativelocation_4 (Variables|/Script/Engine.SceneComponent|GetRelativeLocation _desiredhandscene_2))
  (bind _relativelocation_5 (Variables|/Script/Engine.SceneComponent|GetRelativeLocation _desiredhandscene_3))
  (bind _z (Math|Vector|BreakVector _relativelocation))
  (bind _z_2 (Math|Vector|BreakVector _relativelocation_2))
  (bind (_x _y) (Math|Vector|BreakVector _relativelocation_3))
  (bind (_x_2 _y_2) (Math|Vector|BreakVector _relativelocation_4))
  (bind (_x_3 _y_3) (Math|Vector|BreakVector _relativelocation_5))
  (Transformation|SetRelativeLocation _desiredhandscene_3 (Math|Vector|MakeVector _x_3 _y_3 (Math|Vector|VectorLength (- TargetPoint (Class|KismetMathLibrary|ProjectPointontoPlane TargetPoint (Transformation|GetActorLocation) (Math|Vector|GetUpVector (Transformation|GetActorRotation)))))) false false)
  ;[1 1 1] 손 위치가 버튼에 비해 높은가?
  (if (> _z _z_2)
    (Variables|Default|SetRelRelativeButtonZ 0.0)
    (else
      ;[1 1 1] 그럼 낮은가?
      (if (< _z (.Z (Math|Vector|BreakVector (Variables|/Script/Engine.SceneComponent|GetRelativeLocation (Variables|Default|GetWherePushEnds)))))
        (bind _output_get (Variables|Default|SetRelRelativeButtonZ (* (Variables|Default|GetMoveLength) -1.0)))
        (Transformation|SetRelativeLocation _desiredhandscene_2 (Math|Vector|MakeVector _x_2 _y_2 (+ _output_get (Variables|Default|GetRelativeButtonZ))) false false)
        (else
          (bind _output_get_2 (Variables|Default|SetRelRelativeButtonZ (- _z _z_2))) ; 둘 다 아니면 버튼과 손이 맞닿아 있는것
        ))))
  (Transformation|SetRelativeLocation _button (Math|Vector|MakeVector _x _y (+ _output_get_2 (Variables|Default|GetRelativeButtonZ))) false false))