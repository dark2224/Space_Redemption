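; BP_Controller handles player weapon input, firing regular and guided missiles.
; The Missile input spawns a BP_Missile at the transform of the Missile component on the referenced cockpit.
; The GuidedMissile input spawns nothing: it loops over existing BP_GuidedMissile actors from the GuidedMissile reference's missile array, sets their start flag and unhides them all at once.
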(event EventBeginPlay)

(event EventTick
  (params (DeltaSeconds :type Float%20%28single-precision%29)))

(event Input|ActionEvents|InputActionMissile
  (params (Key :type Key%20Structure :default "AnyKey"))
  (:Pressed
    (Game|SpawnActorfromClass "/Game/Blueprint/Missile/BP_Missile.BP_Missile_C" (Transformation|GetWorldTransform (Variables|/Game/Blueprint/SpaceShip/BP_Cockpit.BP_Cockpit_C|GetMissile (Variables|Default|GetRefCockpit))) "Undefined" 0 0)))

(event Input|ActionEvents|InputActionGuidedMissile
  (params (Key :type Key%20Structure :default "AnyKey"))
  (:Pressed
    (bind _returnvalue (Class|MissileSystem|GetMissileArray (Variables|Default|GetGuidedMissile)))
    (for _array_element _returnvalue
      (bind _asbp_guided_missile (Utilities|Casting|CastToBP_GuidedMissile _array_element))
      (Utilities|Set|StartCheck _asbp_guided_missile true)
      (Rendering|SetActorHiddenInGame _asbp_guided_missile false))))

(fn ConstructionScript)