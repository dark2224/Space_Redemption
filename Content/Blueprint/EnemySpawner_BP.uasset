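; Enemy spawner actor that, once activated, sends waves of enemy fighters against a supplied set of engaging targets.
; Tick accrues a threat budget at a rate that grows as a power curve of elapsed time.
; At randomized intervals it spends that budget, spawning fighters until it cannot afford another.
; Each fighter appears far off within a random cone and receives a random target; MultipleFighters is an unfinished stub.
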(event EventBeginPlay)

(event Collision|EventActorBeginOverlap
  (params (OtherActor :type Actor%20Object%20Reference)))

(event EventTick
  (params (DeltaSeconds :type Float%20%28single-precision%29))
  (if (Variables|Default|GetStarted)
    (bind _output_get (Variables|Default|SetElapsedTime (+ DeltaSeconds (Variables|Default|GetElapsedTime))))
    (bind _output_get_2 (Variables|Default|SetStackedThreatDelta (Math|Float|Power _output_get 0.35)))
    (Variables|Default|SetStackedThreatValue (+ (* _output_get_2 DeltaSeconds) (Variables|Default|GetStackedThreatValue)))
    (if (>= (Variables|Default|GetElapsedTime) (Variables|Default|GetNextSpawn))
      (bind _success (CallFunction|SingleFighter :!label _label))
      (if _success
        (goto _label)
        (else
          (Variables|Default|SetNextSpawn (+ (Variables|Default|GetElapsedTime) (Math|Random|RandomFloatinRange 1.0 7.0))))))))

(fn ConstructionScript)

(fn MakeRandomLocation
  (return (+ (Transformation|GetActorLocation) (* (Math|Vector|GetForwardVector (Math|Rotator|MakeRotator 0.0 (Math|Random|RandomFloatinRange 0.0 6e+01) (Math|Random|RandomFloatinRange -6e+01 6e+01))) (Math|Random|RandomFloatinRange 4e+04 6.5e+04)))))

(fn Activate
  (Variables|Default|SetStarted true))

(fn SingleFighter
  (bind _cost (LocalVariables|GetCost))
  (bind _engagingtargets (Variables|Default|GetEngagingTargets))
  (if (>= (Variables|Default|GetStackedThreatValue) _cost)
    (Variables|Default|SetStackedThreatValue (- (Variables|Default|GetStackedThreatValue) _cost))
    (bind _returnvalue (CallFunction|MakeRandomLocation))
    (bind _returnvalue_2 (Game|SpawnActorfromClass "/Game/Blueprint/EnemyFighter_BP.EnemyFighter_BP_C" (Math|Transform|MakeTransform _returnvalue "0,0.000000, 0") "Undefined" 0 0))
    (Class|AEnemyFighter|SetStategy _returnvalue_2 (Utilities|Array|Get(acopy) _engagingtargets (Math|Random|RandomIntegerinRange 0 (Utilities|Array|LastIndex _engagingtargets))) 1.5e+03 "90.000000,0.000000,0.000000" 4e+03 2.5e+03 1.0 5.0)
    (return (>= (Variables|Default|GetStackedThreatValue) _cost))))

(fn MultipleFighters
  (CallFunction|MakeRandomLocation))

(fn SetEngagingTargets
  (params (EngagingTargets :type Array%20of%20Actor%20Object%20References))
  (Variables|Default|SetEngagingTargets EngagingTargets))