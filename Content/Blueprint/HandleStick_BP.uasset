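; Grabbable control stick, a tangible object that the PilotPawn's left hand moves to produce a normalized facing vector.
; A Tick-driven Idle/Approaching/Interacting state machine starts approach on hand overlap and interaction when the hand is within range and wants to grab.
; While held, real-hand movement deltas accumulate into a coordinate clamped by two marker components and converted to pivot rotation via arcsine.
; When not held, the stick eases back to center.
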(event OnComponentBeginOverlap(ApproachDetector)
  (params (OverlappedComponent :type Primitive%20Component%20Object%20Reference) (OtherActor :type Actor%20Object%20Reference) (OtherComp :type Primitive%20Component%20Object%20Reference) (OtherBodyIndex :type Integer) (bFromSweep :type Boolean) (SweepResult :type Hit%20Result%20Structure%20%28by%20ref%29))
  (|Approach상태초기화 OtherComp OtherComp OtherComp))

(event EventBeginPlay
  (Class|TangibleActor|SetDesiredHandTransform (Variables|Default|GetDesiredHandScene))
  (Variables|Default|SetInteractingAnimation "/Game/Model/Player/LeftAnim/LeftIdle.LeftIdle"))

(event EventTick
  (params (DeltaSeconds :type Float%20%28single-precision%29))
  (bind _returnvalue (Class|TangibleActor|GetStaus))
  (switch Utilities|FlowControl|Switch|SwitchonInteractionStatus _returnvalue
    (:Idle
      (|Idle))
    (:Approaching
      (|접근중조건확인))
    (:Interacting
      (|상호작용중))))

(fn ConstructionScript
  (bind _clamper1 (Variables|Default|GetClamper1))
  (bind _clamper2 (Variables|Default|GetClamper2))
  (bind _relativelocation (Variables|/Script/Engine.SceneComponent|GetRelativeLocation _clamper1))
  (bind _relativelocation_2 (Variables|/Script/Engine.SceneComponent|GetRelativeLocation _clamper2))
  (bind (_x _y) (Math|Vector|BreakVector _relativelocation_2))
  (bind (_x_2 _y_2) (Math|Vector|BreakVector _relativelocation))
  (Variables|Default|SetCoordinateClamper (Math|Vector2D|MakeVector2D (Math|Float|Absolute(Float) (/ (- _x_2 _x) 2.0)) (Math|Float|Absolute(Float) (/ (- _y_2 _y) 2.0)))))

(fn RotatebyCoordinate
  (params (CurrentCoordinate :type Vector%202D%20Structure))
  (bind _sticklength (Variables|Default|GetStickLength))
  (bind _output_get (Variables|Default|SetCurrentCoordinate CurrentCoordinate))
  (Transformation|SetRelativeRotation (Variables|컴포넌트|GetRotateCenter) (Math|Rotator|MakeRotator (Class|KismetMathLibrary|DegAsin (/ (.Y (Math|Vector2D|BreakVector2D _output_get)) _sticklength)) (* (Class|KismetMathLibrary|DegAsin (/ (.X (Math|Vector2D|BreakVector2D _output_get)) _sticklength)) -1.0) 0.0) false false)
  (return _output_get))

(fn ReturntoZeroCoordinate
  (bind _output_get (Variables|Default|SetCurrentReturningFactor (Math|Float|Clamp(Float) (- (Variables|Default|GetCurrentReturningFactor) (* (Variables|Default|GetReturningSpeedRate) (Utilities|Time|GetWorldDeltaSeconds))))))
  (bind _output_get_2 (Variables|Default|SetCurrentCoordinate (* (Variables|Default|GetLastCoordinate) _output_get)))
  (if (> (Math|Vector2D|Vector2DLength _output_get_2) 1.0)
    (Class|HandleStick|SetNormalizedFacingVector (Math|Vector2D|Normalize2D _output_get_2))
    (else
      (Class|HandleStick|SetNormalizedFacingVector)))
  (return _output_get_2))