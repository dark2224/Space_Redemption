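; AI manager Blueprint that steers alliance units and enemy UFOs every Tick.
; The Alliance and Enemy passes clear the shoot flag on each living unit, then feed a per-side TraceMissile result into its Position and MFAngle into its Angle.
; A final AI pass calls Trace for the enemy side at the manager's Speed, with the tracing logic itself defined outside these graphs.
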(event EventBeginPlay)

(event Collision|EventActorBeginOverlap
  (params (OtherActor :type Actor%20Object%20Reference)))

(event EventTick
  (params (DeltaSeconds :type Float%20%28single-precision%29))
  (CallFunction|Alliance)
  (CallFunction|Enemy)
  (CallFunction|AI))

(fn ConstructionScript)

(fn Alliance
  (bind _returnvalue (Class|AIManager|GetAlliance))
  (for _array_element _returnvalue
    (bind _returnvalue_2 (Class|Alliance|GetHp _array_element))
    (if (> _returnvalue_2 0)
      (Utilities|Set|Shoot _array_element false)
      (bind _returnvalue_3 (Class|AIManager|TraceMissile "UNIT_ALLIANCE"))
      (bind _asbp_alliance (Utilities|Casting|CastToBP_Alliance _array_element))
      (Variables|/Game/Blueprint/Alliance/BP_Alliance.BP_Alliance_C|SetPosition _asbp_alliance _returnvalue_3)
      (Variables|/Game/Blueprint/Alliance/BP_Alliance.BP_Alliance_C|SetAngle _asbp_alliance (Variables|Default|Getm_fAngle)))))

(fn Enemy
  (bind _returnvalue (Class|AIManager|GetEnemy))
  (for _array_element _returnvalue
    (bind _returnvalue_2 (Class|Enemy|GetHp _array_element))
    (if (> _returnvalue_2 0)
      (Utilities|Set|Shoot _array_element false)
      (bind _returnvalue_3 (Class|AIManager|TraceMissile "UNIT_ENEMEY"))
      (bind _asbp_ufo (Utilities|Casting|CastToBP_UFO _array_element))
      (Variables|/Game/Blueprint/Enemy/BP_UFO.BP_UFO_C|SetPosition _asbp_ufo _returnvalue_3)
      (Variables|/Game/Blueprint/Enemy/BP_UFO.BP_UFO_C|SetAngle _asbp_ufo (Variables|Default|Getm_fAngle)))))

(fn AI
  (Class|AIManager|Trace "UNIT_ENEMEY" (Variables|AI|GetSpeed)))