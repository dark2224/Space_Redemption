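; Gun actor that animates two rotation pivots, left and right, spinning them continuously in opposite directions.
; Each Tick applies a frame-rate-independent local roll to both pivots, scaled by GetRotationSpeed, whose logic is not defined in this graph.
; SetTouch stores a Touch value, which the visible graphs do not read.
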(event EventBeginPlay)

(event Collision|EventActorBeginOverlap
  (params (OtherActor :type Actor%20Object%20Reference)))

(event EventTick
  (params (DeltaSeconds :type Float%20%28single-precision%29))
  (bind _returnvalue (Class|MiniGun|GetRotationSpeed))
  (Transformation|AddLocalRotation (Variables|Default|GetLeftRotationPivot) (Math|Rotator|MakeRotator (* DeltaSeconds _returnvalue -1.0) 0.0 0.0) false false)
  (Transformation|AddLocalRotation (Variables|Default|GetRightRotationPivot) (Math|Rotator|MakeRotator (* DeltaSeconds _returnvalue 1.0) 0.0 0.0) false false))

(fn ConstructionScript)

(fn SetTouch
  (params (touch :type Touch%20Pad%20BP%20Object%20Reference))
  (Variables|Default|Settouch touch))