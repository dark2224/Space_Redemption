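; BP_HangarDoor is a hangar door that opens and closes based on the player ship's distance.
; BeginPlay passes the door mesh's location to SetPosition.
; Every tick, CheckDoor updates DoorCheck from a distance test between the ship's cockpit and the mesh, gated by a Delay check.
; DoorCheck selects On or Off, which both feed OnOffDoor a state and a frame-rate independent step from MFSpeed.
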(event EventBeginPlay
  (CallFunction|Position))

(event Collision|EventActorBeginOverlap
  (params (OtherActor :type Actor%20Object%20Reference)))

(event EventTick
  (params (DeltaSeconds :type Float%20%28single-precision%29))
  (CallFunction|CheckDoor)
  (if (Variables|Door|GetDoorCheck)
    (CallFunction|On DeltaSeconds)
    (else
      (CallFunction|Off DeltaSeconds))))

(fn ConstructionScript)

(fn CheckDoor
  (bind _returnvalue (Class|EventDoor|Delay))
  (if _returnvalue
    (bind _returnvalue_2 (Class|EventDoor|Distance (Transformation|GetWorldLocation (Variables|/Script/Space_Redemption.PlayerShip|GetCockpit (Variables|Door|GetPlayerShip))) (Transformation|GetWorldLocation (Variables|Default|GetStaticMesh))))
    (Variables|Door|SetDoorCheck _returnvalue_2)))

(fn On
  (params (DeltaSeconds :type Float%20%28single-precision%29))
  (Class|EventDoor|OnOffDoor "DOOR_On" (Transformation|GetWorldLocation (Variables|Default|GetStaticMesh)) (* (Variables|Default|Getm_fSpeed) DeltaSeconds)))

(fn Off
  (params (Delta%20Seconds :type Float%20%28single-precision%29))
  (Class|EventDoor|OnOffDoor "DOOR_Off" (Transformation|GetWorldLocation (Variables|Default|GetStaticMesh)) (* (Variables|Default|Getm_fSpeed) Delta%20Seconds)))

(fn Position
  (Utilities|Set|Position (Transformation|GetWorldLocation (Variables|Default|GetStaticMesh))))